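; BP_EndGame is an end-of-game trigger actor that fires the first time the player overlaps it.
; A one-shot Triggered flag guards the sequence, which plays FMOD audio and calls STOP on the GM game mode.
; After a six-second delay it opens the MainMenu level by object reference.
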(event EventBeginPlay)

(event Collision|EventActorBeginOverlap
  (params (OtherActor :type Actor%20Object%20Reference))
  (Utilities|Casting|CastToBP_Player OtherActor)
  (if (not (Variables|Default|GetTriggered))
    (Variables|Default|SetTriggered true)
    (Class|FMODAudioComponent|Play (Variables|Default|GetFMODAudio))
    (bind _asgm (Utilities|Casting|CastToGM (Game|GetGameMode)))
    (Default|STOP _asgm)
    (Utilities|FlowControl|Delay 6.0)
    (Game|OpenLevel(byObjectReference) "/Game/Menu/MainMenu.MainMenu")))

(event EventTick
  (params (DeltaSeconds :type Float%20%28single-precision%29)))

(fn ConstructionScript)