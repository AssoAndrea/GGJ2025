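; BP_CarrucolaUp is a pulley ("carrucola") actor that rises when the player touches its sphere.
; Sphere overlap plays the Collect component for any actor; for BP_Player it also hides the sphere, sets Broken and stores start and target positions.
; The SaliCorda timeline then lerps the whole actor straight up by a fixed offset, teleporting without sweep.
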(event OnComponentBeginOverlap(Sphere)
  (params (OverlappedComponent :type Primitive%20Component%20Object%20Reference) (OtherActor :type Actor%20Object%20Reference) (OtherComp :type Primitive%20Component%20Object%20Reference) (OtherBodyIndex :type Integer) (bFromSweep :type Boolean) (SweepResult :type Hit%20Result%20Structure%20%28by%20ref%29))
  (bind _returnvalue (Transformation|GetActorLocation))
  (Class|FMODAudioComponent|Play (Variables|Default|Getcollect))
  (Utilities|Casting|CastToBP_Player OtherActor)
  (Rendering|SetVisibility (Variables|Default|GetSphere) false false)
  (Variables|Default|SetBroken true)
  (Variables|Default|SetBeginPos _returnvalue)
  (Variables|Default|SetTargetPos (+ _returnvalue "0.000000,0.000000,500.000000"))
  (CallFunction|EventMuoviCorda))

(event Custom|EventMuoviCorda
  (bind _positiont (Timeline|SaliCorda Play)
    (:Update
      (Transformation|SetActorLocation (Math|Vector|Lerp(Vector) (Variables|Default|GetBeginPos) (Variables|Default|GetTargetPos) _positiont) false true))))

(event EventBeginPlay
  (Variables|Default|SetBroken false))

(fn ConstructionScript)