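; BP_Door is a door actor that opens when its matching key hits it.
; A component hit on the Door casts the other actor to BP_Key and, if it equals the assigned Key while the door is closed, sets Open and fires EventOpenDoor.
; That event plays the Apertura timeline from the start, driving the Pivot component's relative yaw to swing the door open.
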(event OnComponentHit(Door)
  (params (HitComponent :type Primitive%20Component%20Object%20Reference) (OtherActor :type Actor%20Object%20Reference) (OtherComp :type Primitive%20Component%20Object%20Reference) (NormalImpulse :type Vector :default "0, 0, 0") (Hit :type Hit%20Result%20Structure%20%28by%20ref%29))
  (if (not (Variables|Default|GetOpen))
    (bind _asbp_key (Utilities|Casting|CastToBP_Key OtherActor))
    (if (== _asbp_key (Variables|Default|GetKey))
      (Variables|Default|SetOpen true)
      (CallFunction|EventOpenDoor))))

(event Custom|EventOpenDoor
  (bind _rotazione (Timeline|Apertura PlayFromStart)
    (:Update
      (Transformation|SetRelativeRotation (Variables|Default|Getpivot) (Math|Rotator|MakeRotator 0.0 0.0 _rotazione) false false))))

(event EventTick
  (params (DeltaSeconds :type Float%20%28single-precision%29)))

(fn ConstructionScript)