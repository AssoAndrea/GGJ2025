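; Player pawn that moves by bubble jumps, propelling itself opposite the mouse direction on the XZ plane.
; Holding IA_Bubble spawns a BP_Bolla on the head socket, draining the bubble reserve and growing it while the head tracks the cursor.
; Release, or full charge with AutomaticJump, applies a charge-scaled capsule impulse and destroys the bubble.
; A downward trace, paused briefly after release, resets body rotation when grounded and refills the reserve on landing.
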(event Input|EnhancedActionEvents|EnhancedInputActionIA_Bubble
  (params (ActionValue :type Boolean) (ElapsedSeconds :type Float%20%28double-precision%29) (TriggeredSeconds :type Float%20%28double-precision%29) (InputAction :type Input%20Action%20Object%20Reference :default "/Game/ThirdPerson/Input/Actions/IA_Bubble.IA_Bubble"))
  (bind _returnvalue (CallFunction|HaveBubbles))
  (:Started
    (if _returnvalue
      (Variables|Default|SetCharge true)
      (CallFunction|SpawnBolla)))
  (:Completed
    (if _returnvalue
      (if (Variables|Default|GetCharge)
        (CallFunction|BubbleJump)
        (Variables|Default|SetCheckAirDelay true)
        (Utilities|FlowControl|Delay 1.0)
        (Variables|Default|SetCheckAirDelay false)))))

(event EventBeginPlay
  (Variables|/Script/Engine.PlayerController|SetbShowMouseCursor (Game|GetPlayerController 0) true)
  (Variables|Default|SetRemainingBubble (Variables|Config|GetMaxBubble))
  (bind _returnvalue (UserInterface|CreateWidget "/Game/HUD/WBP_GameUI.WBP_GameUI_C"))
  (UserInterface|Viewport|AddtoViewport _returnvalue 0))

(event EventControllerChanged
  (params (OldController :type Controller%20Object%20Reference) (NewController :type Controller%20Object%20Reference))
  (bind _asplayer_controller (Utilities|Casting|CastToPlayerController NewController))
  (Input|AddMappingContext (PlayerController|LocalPlayerSubsystems|GetEnhancedInputLocalPlayerSubsystem _asplayer_controller) "/Game/ThirdPerson/Input/IMC_Default.IMC_Default" 0 "(bIgnoreAllPressedKeysUntilRelease=True,bForceImmediately=False,bNotifyUserSettings=False)"))

(event EventTick
  (params (DeltaSeconds :type Float%20%28single-precision%29))
  (Utilities|FlowControl|Sequence
    (:then_0
      (if (Variables|Default|GetCharge)
        (CallFunction|ChargeBolla DeltaSeconds)))
    (:then_1
      (if (not (Variables|Default|GetCheckAirDelay))
        (CallFunction|CheckIsinAir)
        (if (not (Variables|Default|GetIsInAir))
          (Transformation|SetRelativeRotation (Variables|Default|GetStaticMesh) "0, 0, 0" false false)
          (if true
            _))))))

(event Collision|EventActorBeginOverlap
  (params (OtherActor :type Actor%20Object%20Reference)))

(fn ConstructionScript)

(fn BubbleJump
  (bind _mousedirection (Variables|Default|GetMouseDirection))
  (Physics|AddImpulse (Variables|Default|GetCapsule) (* (Variables|Default|GetMouseDirection) (* (/ (Variables|Default|GetCurrentUsedBubble) (Variables|Default|GetMaxSingleBubble)) -1.0 (Variables|Config|GetMaxBubbleForce))) "None" true)
  (Variables|Default|SetCharge false)
  (Variables|Default|SetCurrentUsedBubble 0.0)
  (Actor|DestroyActor (Variables|Default|GetBolla))
  (CallFunction|RotateBody _mousedirection)
  (CallFunction|RotateTesta _mousedirection))

(fn SpawnBolla
  (bind _returnvalue (Game|SpawnActorfromClass "/Game/Blueprints/BP_Bolla.BP_Bolla_C" (Math|Conversions|ToTransform(Vector) (Transformation|GetSocketLocation (Variables|Default|GetTesta) "Spawn")) "Undefined" "MultiplyWithRoot" 0 0))
  (Transformation|AttachComponentToComponent _returnvalue (Variables|Default|GetTesta) "Spawn" "SnapToTarget" "KeepRelative" "KeepWorld" true)
  (Variables|Default|SetBolla _returnvalue))

(fn ChargeBolla
  (params (DeltaTIme :type Float%20%28double-precision%29))
  (bind _returnvalue (Game|GetPlayerController 0))
  (bind _maxsinglebubble (Variables|Default|GetMaxSingleBubble))
  (bind _chargespeed (Variables|Config|GetChargeSpeed))
  (bind _worlddirection (Game|Player|ConvertMouseLocationToWorldSpace _returnvalue))
  (bind _returnvalue_2 (* DeltaTIme _chargespeed))
  (bind _output_get (Variables|Default|SetCurrentUsedBubble (Math|Float|Clamp(Float) (+ (Variables|Default|GetCurrentUsedBubble) _returnvalue_2) 0.0 _maxsinglebubble)))
  (bind _output_get_2 (Variables|Default|SetRemainingBubble (Math|Float|Clamp(Float) (- (Variables|Default|GetRemainingBubble) _returnvalue_2) 0.0 (Variables|Config|GetMaxBubble))))
  (bind _output_get_3 (Variables|Default|SetMouseDirection (Math|Vector|MakeVector (.x _worlddirection) 0.0 (.z _worlddirection))))
  (CallFunction|RotateTesta _output_get_3)
  (if (and (>= _output_get _maxsinglebubble) (Variables|Default|GetAutomaticJump))
    (CallFunction|BubbleJump)
    (else
      (Default|SetScaleMult (Variables|Default|GetBolla) (Math|Float|Clamp(Float) (/ (Variables|Default|GetCurrentUsedBubble) (Variables|Default|GetMaxSingleBubble)))))))

(fn CheckIsinAir
  (bind _returnvalue (Math|Vector|VectorDown))
  (bind _capsule (Variables|Default|GetCapsule))
  (bind _capsule_2 (Variables|Default|GetCapsule))
  (bind _returnvalue_2 (Components|Capsule|GetScaledCapsuleHalfHeight _capsule))
  (bind _returnvalue_3 (Transformation|GetWorldLocation _capsule_2))
  (bind _returnvalue_4 (* _returnvalue _returnvalue_2))
  (bind _returnvalue_5 (+ _returnvalue_3 _returnvalue_4))
  (bind _returnvalue_6 (Collision|LineTraceByChannel _returnvalue_5 (+ _returnvalue_5 (* (Math|Vector|VectorDown) 1e+01)) "TraceTypeQuery1" false 0 "ForDuration"))
  (Utilities|FlowControl|Sequence
    (:then_0
      (if _returnvalue_6
        (if (!= (Variables|Default|GetIsInAir) (not _returnvalue_6))
          (Variables|Default|SetRemainingBubble (Variables|Config|GetMaxBubble)))))
    (:then_1
      (Variables|Default|SetIsInAir (not _returnvalue_6)))))

(fn RotateBody
  (params (Direction :type Vector))
  (Transformation|SetRelativeRotation (Variables|Default|GetStaticMesh) (Math|Rotator|MakeRotfromZY (* Direction -1.0) (Math|Vector|VectorUp)) false false))

(fn RotateTesta
  (params (Direction :type Vector%20%28by%20ref%29))
  (Transformation|SetWorldRotation (Variables|Default|GetTesta) (Math|Rotator|MakeRotfromZY Direction (Math|Vector|VectorUp)) false false))

(fn HaveBubbles
  (return (> (Variables|Default|GetRemainingBubble) 0)))