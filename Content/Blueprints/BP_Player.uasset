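; Player character that launches itself with charged bubble jumps in the XZ plane, opposite to the mouse direction.
; Holding IA_Bubble grows an attached BP_Bolla and aims the head pivot; release, or optionally full charge, applies the impulse and rotates the body.
; Each jump spends a bubble; a downward ground trace, paused briefly after release-triggered jumps, refills them and updates the HUD on landing.
; Also creates the game UI and pause menu.
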(event Input|EnhancedActionEvents|EnhancedInputActionPause
  (params (ActionValue :type Boolean) (ElapsedSeconds :type Float%20%28double-precision%29) (TriggeredSeconds :type Float%20%28double-precision%29) (InputAction :type Input%20Action%20Object%20Reference :default "/Game/ThirdPerson/Input/Actions/Pause.Pause"))
  (Game|SetGamePaused true)
  (bind _returnvalue (UserInterface|CreateWidget "/Game/Menu/PauseMenuWidget.PauseMenuWidget_C"))
  (UserInterface|Viewport|AddtoViewport _returnvalue 0))

(event Input|EnhancedActionEvents|EnhancedInputActionIA_Bubble
  (params (ActionValue :type Boolean) (ElapsedSeconds :type Float%20%28double-precision%29) (TriggeredSeconds :type Float%20%28double-precision%29) (InputAction :type Input%20Action%20Object%20Reference :default "/Game/ThirdPerson/Input/Actions/IA_Bubble.IA_Bubble"))
  (bind _returnvalue (CallFunction|HaveBubbles))
  (:Started
    (if _returnvalue
      (Variables|Default|SetCharge true)
      (CallFunction|SpawnBolla)))
  (:Completed
    (if _returnvalue
      (if (Variables|Default|GetCharge)
        (CallFunction|BubbleJump)
        (Variables|Default|SetCheckAirDelay true)
        (Utilities|FlowControl|Delay 0.2)
        (Variables|Default|SetCheckAirDelay false)))))

(event EventBeginPlay
  (Variables|/Script/Engine.PlayerController|SetbShowMouseCursor (Game|GetPlayerController 0) true)
  (Variables|Default|SetRemainingBubble (Variables|Config|GetMaxBubble))
  (bind _returnvalue (UserInterface|CreateWidget "/Game/HUD/WBP_GameUI.WBP_GameUI_C"))
  (UserInterface|Viewport|AddtoViewport _returnvalue 0)
  (Variables|Default|SetHUD _returnvalue))

(event EventControllerChanged
  (params (OldController :type Controller%20Object%20Reference) (NewController :type Controller%20Object%20Reference))
  (bind _asplayer_controller (Utilities|Casting|CastToPlayerController NewController))
  (Input|AddMappingContext (PlayerController|LocalPlayerSubsystems|GetEnhancedInputLocalPlayerSubsystem _asplayer_controller) "/Game/ThirdPerson/Input/IMC_Default.IMC_Default" 0 "(bIgnoreAllPressedKeysUntilRelease=True,bForceImmediately=False,bNotifyUserSettings=False)"))

(event EventTick
  (params (DeltaSeconds :type Float%20%28single-precision%29))
  (Utilities|FlowControl|Sequence
    (:then_0
      (if (Variables|Default|GetCharge)
        (CallFunction|ChargeBolla DeltaSeconds)))
    (:then_1
      (if (not (Variables|Default|GetCheckAirDelay))
        (CallFunction|CheckIsinAir)
        (if (not (Variables|Default|GetIsInAir))
          (Transformation|SetRelativeRotation (Variables|Default|GetPivotCorpo) "0.000000,90.000000,0.000000" false false))))))

(event Collision|EventActorBeginOverlap
  (params (OtherActor :type Actor%20Object%20Reference)))

(fn ConstructionScript)

(fn BubbleJump
  (bind _remainingbubble (Variables|Default|GetRemainingBubble))
  (bind _maxforce (Variables|Config|GetMaxForce))
  (bind _mousedirection (Variables|Default|GetMouseDirection))
  (Physics|AddImpulse (Variables|Default|GetCapsule) (* (Variables|Default|GetMouseDirection) (* (Math|Float|Clamp(Float) (Variables|Default|GetForce) (Variables|Config|GetMinForce) _maxforce) -1.0)) "None" true)
  (Variables|Default|SetCharge false)
  (Variables|Default|SetNormalizedForce (/ (Variables|Default|GetForce) _maxforce))
  (Variables|Default|SetForce 0.0)
  (Actor|DestroyActor (Variables|Default|GetBolla))
  (CallFunction|RotateBody _mousedirection)
  (CallFunction|RotateTesta _mousedirection)
  (Math|Integer|DecrementInt _remainingbubble
    (:%20%20
      (Default|SetBubbleCounter (Variables|Default|GetHUD) _remainingbubble)
      (CallFunction|SetIsinAir true))))

(fn SpawnBolla
  (bind _returnvalue (Game|SpawnActorfromClass "/Game/Blueprints/BP_Bolla.BP_Bolla_C" (Math|Conversions|ToTransform(Vector) (Transformation|GetSocketLocation (Variables|Default|GetSkeletalMesh) "Spawn")) "Undefined" "MultiplyWithRoot" 0 0))
  (Transformation|AttachComponentToComponent _returnvalue (Variables|Default|GetSkeletalMesh) "Spawn" "SnapToTarget" "KeepRelative" "KeepWorld" true)
  (Variables|Default|SetBolla _returnvalue))

(fn ChargeBolla
  (params (DeltaTIme :type Float%20%28double-precision%29))
  (bind _returnvalue (Game|GetPlayerController 0))
  (bind _maxforce (Variables|Config|GetMaxForce))
  (bind _worlddirection (Game|Player|ConvertMouseLocationToWorldSpace _returnvalue))
  (bind _output_get (Variables|Default|SetForce (+ (Variables|Default|GetForce) (* (Variables|Config|GetChargeSpeed) DeltaTIme))))
  (bind _output_get_2 (Variables|Default|SetMouseDirection (Math|Vector|MakeVector (.x _worlddirection) 0.0 (.z _worlddirection))))
  (CallFunction|RotateTesta _output_get_2)
  (if (and (>= _output_get _maxforce) (Variables|Default|GetAutomaticJump))
    (CallFunction|BubbleJump)
    (else
      (Default|SetScaleMult (Variables|Default|GetBolla) (Math|Float|Clamp(Float) (/ _output_get _maxforce))))))

(fn CheckIsinAir
  (bind _returnvalue (Math|Vector|VectorDown))
  (bind _capsule (Variables|Default|GetCapsule))
  (bind _capsule_2 (Variables|Default|GetCapsule))
  (bind _returnvalue_2 (Components|Capsule|GetScaledCapsuleHalfHeight _capsule))
  (bind _returnvalue_3 (Transformation|GetWorldLocation _capsule_2))
  (bind _returnvalue_4 (* _returnvalue _returnvalue_2))
  (bind _returnvalue_5 (+ _returnvalue_3 _returnvalue_4))
  (bind _returnvalue_6 (Collision|LineTraceByChannel _returnvalue_5 (+ _returnvalue_5 (* (Math|Vector|VectorDown) 2e+01)) "TraceTypeQuery1" false 0 "ForOneFrame"))
  (CallFunction|SetIsinAir (not _returnvalue_6)))

(fn RotateBody
  (params (Direction :type Vector))
  (Transformation|SetRelativeRotation (Variables|Default|GetPivotCorpo) (Math|Rotator|MakeRotfromZY (* Direction -1.0) (Math|Vector|VectorUp)) false false))

(fn RotateTesta
  (params (Direction :type Vector%20%28by%20ref%29))
  (Transformation|SetWorldRotation (Variables|Default|GetPivotBecco) (Class|KismetMathLibrary|MakeRotfromYZ (* Direction -1.0) (Math|Vector|VectorUp)) false false))

(fn HaveBubbles
  (return (> (Variables|Default|GetRemainingBubble) 0)))

(fn SetIsinAir
  (params (NewVal :type Boolean))
  (if (and (not NewVal) (!= (Variables|Default|GetIsInAir) NewVal))
    (bind _output_get (Variables|Default|SetRemainingBubble (Variables|Config|GetMaxBubble)))
    (Default|SetBubbleCounter (Variables|Default|GetHUD) _output_get))
  (Variables|Default|SetIsInAir NewVal))