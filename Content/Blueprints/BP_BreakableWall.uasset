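; Breakable wall actor that shatters when the player hits it hard enough.
; On a mesh hit by BP_Player, it passes the normal impulse through the actor transform's TransformDirection and compares the absolute X to ForceNeeded.
; Above that threshold it destroys the mesh, plays Breackwall and spawns a wood particle effect.
; Debug prints report hits and force; the Broken guard is read but never set here.
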(event OnComponentHit(Mesh)
  (params (HitComponent :type Primitive%20Component%20Object%20Reference) (OtherActor :type Actor%20Object%20Reference) (OtherComp :type Primitive%20Component%20Object%20Reference) (NormalImpulse :type Vector :default "0, 0, 0") (Hit :type Hit%20Result%20Structure%20%28by%20ref%29))
  (bind _self self)
  (bind _returnvalue (Transformation|GetActorTransform _self))
  (bind _returnvalue_2 (Math|Transform|TransformDirection _returnvalue NormalImpulse))
  (bind _x (Math|Vector|BreakVector _returnvalue_2))
  (bind _returnvalue_3 (Math|Float|Absolute(Float) _x))
  (Development|PrintString "HIT")
  (if (not (Variables|Default|GetBroken))
    (Utilities|Casting|CastToBP_Player OtherActor)
    (Development|PrintString (Utilities|String|ToString(Float) _returnvalue_3))
    (if (> _returnvalue_3 (Variables|Default|GetForceNeeded))
      (Components|DestroyComponent (Variables|Default|GetMesh))
      (Class|FMODAudioComponent|Play (Variables|Default|Getbreackwall))
      (Effects|SpawnEmitteratLocation "/Game/Realistic_Starter_VFX_Pack_Vol2/Particles/Hit/P_Wood.P_Wood" (.Location (Math|Transform|BreakTransform _returnvalue))))))

(event EventBeginPlay)

(event Collision|EventActorBeginOverlap
  (params (OtherActor :type Actor%20Object%20Reference)))

(event EventTick
  (params (DeltaSeconds :type Float%20%28single-precision%29)))

(fn ConstructionScript)